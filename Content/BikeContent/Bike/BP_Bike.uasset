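; Player-driven Chaos vehicle bike that also owns the game's main menu, HUD and race timer display.
; BeginPlay pauses behind the menu until Start creates the HUD, caches the movement component and starts a looping CheckDrift timer.
; Axis inputs drive vehicle and camera, R resets the bike, and Tick maps RPM to engine audio.
; CheckDrift traces the surface under the dirt effect, scaling particle rates by wheel spin; StartRace/StopRace control the HUD timer.
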(event `SettingButtonClick`
  (bind _returnvalue (`|CreateWidget` "/Game/W_MainMenu/Setting_W.Setting_W_C"))
  (`UserWidget.AddToViewport` _returnvalue 0))

(event `StartGame`
  (bind _returnvalue (`GameplayStatics.GetPlayerController` 0))
  (`WidgetLayoutLibrary.RemoveAllWidgets`)
  (`WidgetBlueprintLibrary.SetInputMode_GameOnly` _returnvalue)
  (set `PlayerController.bShowMouseCursor` false _returnvalue)
  (`GameplayStatics.SetGamePaused` false)
  (bind _returnvalue_2 (`|CreateWidget` "/Game/BikeContent/Widgets/W_HUD.W_HUD_C" null self))
  (bind _output_get (set `self.HudWidget` _returnvalue_2))
  (`UserWidget.AddToViewport` _output_get 0)
  (bind _aschaos_wheeled_vehicle_movement_component (cast `ChaosWheeledVehicleMovementComponent` (`self.VehicleMovementComponent`)))
  (set `self.MovementComponent` _aschaos_wheeled_vehicle_movement_component)
  (`KismetSystemLibrary.K2_SetTimer` self "CheckDrift" 0.01 true))

(event `self.ReceiveBeginPlay`
  (bind _returnvalue (`GameplayStatics.GetPlayerController` 0))
  (bind _returnvalue_2 (`|CreateWidget` "/Game/W_MainMenu/MainMenu_w.MainMenu_w_C"))
  (bind _output_get (set `self.MainMenu_Ref` _returnvalue_2))
  (`UserWidget.AddToViewport` _output_get 0)
  (`GameplayStatics.SetGamePaused` true)
  (`WidgetBlueprintLibrary.SetInputMode_UIOnlyEx` _returnvalue (`self.MainMenu_Ref`))
  (set `PlayerController.bShowMouseCursor` true _returnvalue)
  (add `Button.OnClicked` (`/Game/W_MainMenu/MainMenu_w.Setting_Button` (`self.MainMenu_Ref`)) (delegate `SettingButtonClick`))
  (add `Button.OnClicked` (`/Game/W_MainMenu/MainMenu_w.Start_Button` (`self.MainMenu_Ref`)) (delegate `StartGame`)))

(event `InputAxis|MoveForward`
  (params (AxisValue :type "Float (single-precision)"))
  (`ChaosVehicleMovementComponent.SetThrottleInput` (`self.VehicleMovementComponent`) AxisValue))

(event `InputAxis|MoveBack/Break`
  (params (AxisValue :type "Float (single-precision)"))
  (`ChaosVehicleMovementComponent.SetBrakeInput` (`self.VehicleMovementComponent`) AxisValue))

(event `InputAxis|TurnLeft`
  (params (AxisValue :type "Float (single-precision)"))
  (`ChaosVehicleMovementComponent.SetSteeringInput` (`self.VehicleMovementComponent`) AxisValue))

(event `InputAxis|LookRight`
  (params (AxisValue :type "Float (single-precision)"))
  (`self.AddControllerYawInput` AxisValue))

(event `InputAxis|LookUp`
  (params (AxisValue :type "Float (single-precision)"))
  (`self.AddControllerPitchInput` AxisValue))

(event `Key|R`
  (params (Key :type "Key Structure"))
  (bind (_returnvalue_x _returnvalue_y _returnvalue_z) (`KismetMathLibrary.BreakVector` (`self.K2_GetActorLocation`)))
  (:`Pressed`
    (`ChaosVehicleMovementComponent.ResetVehicle` (`self.VehicleMovementComponent`))
    (`self.K2_SetActorLocation` (`KismetMathLibrary.MakeVector` _returnvalue_x _returnvalue_y (+ _returnvalue_z 30.0)) false true)))

(event `self.ReceiveTick`
  (params (DeltaSeconds :type "Float (single-precision)"))
  (`self.UpdateEngineSound`))

(event `UpdateEngineSound`
  (bind (_enginerpm _maxenginerpm) (`self.GetEngineRPM`))
  (bind _audio (`self.Audio`))
  (bind _returnvalue (/ _enginerpm _maxenginerpm))
  (`AudioParameterControllerInterface.SetFloatParameter` _audio "RPM" (`KismetMathLibrary.Lerp` 0.0 2.0 _returnvalue))
  (`AudioComponent.SetPitchMultiplier` _audio (`KismetMathLibrary.FClamp` (* (+ _returnvalue 0.2) 1.4) 0.0 2.0)))

(fn `CheckDrift`
  (bind _movementcomponent (`self.MovementComponent`))
  (bind _returnvalue (`SceneComponent.K2_GetComponentLocation` (`self.Dirt`)))
  (bind _returnvalue_2 (`ChaosVehicleWheel.GetWheelAngularVelocity` (`|GetArrayItem` (`ChaosWheeledVehicleMovementComponent.Wheels` _movementcomponent) 1)))
  (if (`ChaosWheeledVehicleMovementComponent.BreakWheelStatus` (`ChaosWheeledVehicleMovementComponent.GetWheelState` _movementcomponent 1))
    (bind _outhit (`KismetSystemLibrary.LineTraceSingle` :`Start` _returnvalue :`End` (+ _returnvalue (0.0 0.0 -10.0)) :`TraceChannel` "TraceTypeQuery1" :`DrawTime` 0.0))
    (`FXSystemComponent.SetFloatParameter` (`self.Dirt`) "DustSpawnRate" (`KismetMathLibrary.Lerp` 0.0 (select `EPhysicalSurface` (`GameplayStatics.GetSurfaceType` _outhit) :`SurfaceType_Default` 50.0 :`SurfaceType1` 50.0) (/ _returnvalue_2 100.0)))
    (`FXSystemComponent.SetFloatParameter` (`self.Dirt`) "GriftSpawnRate" (`KismetMathLibrary.Lerp` 0.0 (select `EPhysicalSurface` (`GameplayStatics.GetSurfaceType` _outhit) :`SurfaceType2` 500.0) (/ _returnvalue_2 50.0)))
    (else
      (`FXSystemComponent.SetFloatParameter` (`self.Dirt`) "DustSpawnRate" 0.0)
      (`FXSystemComponent.SetFloatParameter` (`self.Dirt`) "GriftSpawnRate" 0.0))))

(fn `GetEngineRPM`
  (returns (EngineRPM :type "Float (double-precision)") (MaxEngineRPM :type "Float (single-precision)"))
  (bind _movementcomponent (`self.MovementComponent`))
  (return (`ChaosWheeledVehicleMovementComponent.GetEngineRotationSpeed` _movementcomponent) (`ChaosWheeledVehicleMovementComponent.GetEngineMaxRotationSpeed` _movementcomponent)))

(fn `StartRace`
  (bind _w_raceinterface (`/Game/BikeContent/Widgets/W_HUD.W_RaceInterface` (`self.HudWidget`)))
  (`Widget.SetVisibility` _w_raceinterface "Visible")
  (bind _returnvalue (`KismetSystemLibrary.K2_SetTimer` _w_raceinterface "UpdateTimer" 0.01 true))
  (set `self.RaceTimer` _returnvalue))

(fn `StopRace`
  (bind _hudwidget (`self.HudWidget`))
  (bind _racetimer (`self.RaceTimer`))
  (`UserWidget.PlayAnimation` _hudwidget (`/Game/BikeContent/Widgets/W_HUD.Fade` _hudwidget) 0.0 1 "Forward" 1.0 false)
  (`KismetSystemLibrary.K2_PauseTimerHandle` _racetimer)
  (`KismetSystemLibrary.K2_ClearAndInvalidateTimerHandle` _racetimer))

(fn `UserConstructionScript`)