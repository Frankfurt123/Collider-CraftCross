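; Spline-based race track for bikes that handles checkpoints, laps, and race start and finish.
; The construction script places a box trigger and point light at each spline point.
; The first box starts the race, counts laps and stops it after the last, while other checkpoints unbind on overlap and arm the next, enforcing order.
; Light intensity highlights the next checkpoint, and progress is written to the bike's HUD.
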(event `RegularPoint`
  (params (OverlappedComponent :type "PrimitiveComponent Object Reference") (OtherActor :type "Actor Object Reference") (OtherComp :type "PrimitiveComponent Object Reference") (OtherBodyIndex :type Integer) (bFromSweep :type Boolean) (SweepResult :type "HitResult Structure (by ref)"))
  (bind _lights (`self.Lights`))
  (bind _asbp_bike (cast `/Game/BikeContent/Bike/BP_Bike` OtherActor))
  (clear `PrimitiveComponent.OnComponentBeginOverlap` OverlappedComponent)
  (bind _result (`/Engine/EditorBlueprintResources/StandardMacros.IncrementInt` (`self.CurrentPoint`))
    (:`  `
      (`TextBlock.SetText` (`/Game/BikeContent/Widgets/W_RaceInterface.TextBlock_96` (`/Game/BikeContent/Widgets/W_HUD.W_RaceInterface` (`/Game/BikeContent/Bike/BP_Bike.HudWidget` _asbp_bike))) (`|FormatText` "Checkpoints: {n}/{n1}" (- (`self.CurrentPoint`) 1) (`SplineComponent.GetNumberOfSplinePoints` (`self.Spline`))))
      (add `PrimitiveComponent.OnComponentBeginOverlap` (`|GetArrayItem` (`self.Points`) _result) (`|CreateDelegate` self :!event `RegularPoint`))
      (`LightComponent.SetIntensity` (`|GetArrayItem` _lights _result) 5000.0)
      (`LightComponent.SetIntensity` (`|GetArrayItem` _lights (- _result 1)) 0.0)
      (if (== _result (`SplineComponent.GetNumberOfSplinePoints` (`self.Spline`)))
        (`LightComponent.SetIntensity` (`|GetArrayItem` (`self.Lights`)) 5000.0)))))

(event `self.ReceiveBeginPlay`
  (add `PrimitiveComponent.OnComponentBeginOverlap` (`|GetArrayItem` (`self.Points`)) (delegate `FirstPoint`)))

(event `FirstPoint`
  (params (OverlappedComponent :type "PrimitiveComponent Object Reference") (OtherActor :type "Actor Object Reference") (OtherComp :type "PrimitiveComponent Object Reference") (OtherBodyIndex :type Integer) (bFromSweep :type Boolean) (SweepResult :type "HitResult Structure (by ref)"))
  (bind _lights (`self.Lights`))
  (bind _currentpoint (`self.CurrentPoint`))
  (bind _asbp_bike (cast `/Game/BikeContent/Bike/BP_Bike` OtherActor))
  (if (`self.IsRaceStarted`)
    (if (== (`SplineComponent.GetNumberOfSplinePoints` (`self.Spline`)) _currentpoint)
      (if (== (`self.LapsMax`) (`self.LapsCurrent`))
        (`/Game/BikeContent/Bike/BP_Bike.StopRace` _asbp_bike)
        (bind _output_get (set `self.CurrentPoint` (+ _currentpoint 1)))
        (bind _textblock_96 (`/Game/BikeContent/Widgets/W_RaceInterface.TextBlock_96` (`/Game/BikeContent/Widgets/W_HUD.W_RaceInterface` (`/Game/BikeContent/Bike/BP_Bike.HudWidget` _asbp_bike))))
        (`TextBlock.SetText` _textblock_96 (`|FormatText` "Checkpoints: {n}/{n1}" (- (`self.CurrentPoint`) 1) (`SplineComponent.GetNumberOfSplinePoints` (`self.Spline`))))
        (`PrimitiveComponent.SetCollisionEnabled` OverlappedComponent "NoCollision")
        (set `self.IsRaceStarted` false)
        (`LightComponent.SetIntensity` (`|GetArrayItem` _lights (- _output_get 1)) 0.0)
        (`LightComponent.SetIntensity` (`|GetArrayItem` (`self.Lights`)) 0.0)
        (bind _textblock_96_2 (`/Game/BikeContent/Widgets/W_RaceInterface.TextBlock_96` (`/Game/BikeContent/Widgets/W_HUD.W_RaceInterface` (`/Game/BikeContent/Bike/BP_Bike.HudWidget` _asbp_bike))))
        (`TextBlock.SetText` _textblock_96_2 (`|FormatText` "Checkpoints: {n}/{n1}" (- (`self.CurrentPoint`) 1) (`SplineComponent.GetNumberOfSplinePoints` (`self.Spline`))))
        (else
          (`/Engine/EditorBlueprintResources/StandardMacros.IncrementInt` (`self.LapsCurrent`)
            (:`  `
              (add `PrimitiveComponent.OnComponentBeginOverlap` (`|GetArrayItem` (`self.Points`) 1) (`|CreateDelegate` self :!event `RegularPoint`))
              (`LightComponent.SetIntensity` (`|GetArrayItem` (`self.Lights`) 1) 5000.0)
              (set `self.CurrentPoint` 1)
              (`TextBlock.SetText` (`/Game/BikeContent/Widgets/W_RaceInterface.TextBlock` (`/Game/BikeContent/Widgets/W_HUD.W_RaceInterface` (`/Game/BikeContent/Bike/BP_Bike.HudWidget` _asbp_bike))) (`|FormatText` "Laps: {n}/{n1}" (`self.LapsCurrent`) (`self.LapsMax`)))
              (`TextBlock.SetText` _textblock_96 (`|FormatText` "Checkpoints: {n}/{n1}" (- (`self.CurrentPoint`) 1) (`SplineComponent.GetNumberOfSplinePoints` (`self.Spline`))))
              (`LightComponent.SetIntensity` (`|GetArrayItem` (`self.Lights`)) 0.0))))))
    (else
      (`/Game/BikeContent/Bike/BP_Bike.StartRace` _asbp_bike)
      (bind _output_get_2 (set `self.CurrentPoint` 1))
      (`TextBlock.SetText` _textblock_96_2 (`|FormatText` "Checkpoints: {n}/{n1}" (- (`self.CurrentPoint`) 1) (`SplineComponent.GetNumberOfSplinePoints` (`self.Spline`))))
      (set `self.IsRaceStarted` true)
      (add `PrimitiveComponent.OnComponentBeginOverlap` (`|GetArrayItem` (`self.Points`) _output_get_2) (`|CreateDelegate` self :!event `RegularPoint`))
      (`LightComponent.SetIntensity` (`|GetArrayItem` _lights _output_get_2) 5000.0))))

(fn `UserConstructionScript`
  (bind _spline (`self.Spline`))
  (for _index (range (`SplineComponent.GetNumberOfSplinePoints` _spline))
    (bind _returnvalue (`SplineComponent.GetLocationAtSplinePoint` _spline _index "Local"))
    (bind _returnvalue_2 (`AddComponent|NODE_AddBoxComponent-0` :`RelativeTransform` (`KismetMathLibrary.MakeTransform` _returnvalue (`SplineComponent.GetRotationAtSplinePoint` _spline _index "Local") (`self.BoxScale`))))
    (`KismetArrayLibrary.Array_AddUnique` (`self.Points`) _returnvalue_2)
    (bind _returnvalue_3 (`AddComponent|NODE_AddPointLightComponent-0` :`RelativeTransform` (`KismetMathLibrary.MakeTransform` _returnvalue)))
    (`KismetArrayLibrary.Array_AddUnique` (`self.Lights`) _returnvalue_3)))